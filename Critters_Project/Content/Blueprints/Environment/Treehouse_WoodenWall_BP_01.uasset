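; Treehouse wooden wall Blueprint that builds a modular wall of configurable length from static mesh pieces.
; The construction script adds a mesh component per piece, spaced at fixed intervals along negative local X, using the basic wall mesh for all but the last and an end mesh to cap the run.
; Each component is stored in a wall array; the event graph has no active logic.
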(fn `UserConstructionScript`
  (bind _numberofwallpieces (`self.numberOfWallPieces`))
  (bind _wall_arr (`self.wall_Arr`))
  (bind _returnvalue (- _numberofwallpieces 1))
  (for _index (range (+ (- _numberofwallpieces 2) 1))
    (bind _returnvalue_2 (`AddComponent|NODE_AddStaticMeshComponent-0` :`RelativeTransform` (`KismetMathLibrary.Conv_VectorToTransform` (`KismetMathLibrary.MakeVector` (* (`KismetMathLibrary.Conv_IntToDouble` _index) -100.0)))))
    (`StaticMeshComponent.SetStaticMesh` _returnvalue_2 (`self.WallBasic`))
    (`KismetArrayLibrary.Array_Set` _wall_arr _index _returnvalue_2 true))
  (bind _returnvalue_3 (`AddComponent|NODE_AddStaticMeshComponent-1` :`RelativeTransform` (`KismetMathLibrary.Conv_VectorToTransform` (`KismetMathLibrary.MakeVector` (* (`KismetMathLibrary.Conv_IntToDouble` _returnvalue) -100.0)))))
  (`StaticMeshComponent.SetStaticMesh` _returnvalue_3 (`self.WallEnd`))
  (`KismetArrayLibrary.Array_Set` _wall_arr _returnvalue _returnvalue_3 true))