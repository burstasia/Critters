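; Environment tree Blueprint that lets each placed instance show one of three tree variants.
; The construction script compares the WhichTree enum and makes the matching component, TreeEnv01, TreeEnv02 or TreeEnv03, visible.
; It only turns visibility on and never hides the other variants itself.
; The event graph has no active logic.
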(fn `UserConstructionScript`
  (`|ExecutionSequence`
    (:`then_0`
      (if (`|EnumEquality` (`self.Which Tree`) "NewEnumerator0")
        (`SceneComponent.SetVisibility` (`self.Tree_Env_01`) true false)))
    (:`then_1`
      (if (`|EnumEquality` (`self.Which Tree`) "NewEnumerator1")
        (`SceneComponent.SetVisibility` (`self.Tree_Env_02`) true false)))
    (:`then_2`
      (if (`|EnumEquality` (`self.Which Tree`) "NewEnumerator2")
        (`SceneComponent.SetVisibility` (`self.Tree_Env_03`) true false)))))