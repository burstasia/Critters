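; Base room actor Blueprint that marks a box volume and registers itself as the room reference when the player enters it.
; The construction script sizes the box extent from XSize, YSize and ZSize.
; On overlap by the first player controller's pawn, it runs an actor class lookup and calls SetRoomRef with itself.
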(event `self.ReceiveActorBeginOverlap`
  (params (OtherActor :type "Actor Object Reference"))
  (if (== OtherActor (`Controller.K2_GetPawn` (`GameplayStatics.GetPlayerController` 0)))
    (bind _outactors (`GameplayStatics.GetAllActorsOfClass` null))
    (`self.SetRoomRef` self)))

(event `self.ReceiveTick`
  (params (DeltaSeconds :type "Float (single-precision)")))

(fn `UserConstructionScript`
  (`BoxComponent.SetBoxExtent` (`self.Box`) (`KismetMathLibrary.MakeVector` (`self.XSize`) (`self.YSize`) (`self.ZSize`)) true))