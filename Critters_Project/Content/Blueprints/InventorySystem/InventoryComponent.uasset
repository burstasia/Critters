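; Inventory component that shows and hides an inventory window on the player's HUD.
; ToggleInventory removes the window if it exists, otherwise creates one with the component passed in as its Inventory.
; The new widget is added to the HUD canvas of player 0's MyPlayerController, auto-sized and anchored bottom-left.
; The event graph is empty, and a position-setting call is left unconnected.
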(fn `ToggleInventory`
  (`self.InventoryWindow`
    (:`then`
      (`Widget.RemoveFromParent` (`self.InventoryWindow`))
      (set `self.InventoryWindow` null))
    (:`else`
      (bind _returnvalue (`|CreateWidget` "/Game/Blueprints/InventorySystem/InventoryUI/InventoryWindow.InventoryWindow_C" null self))
      (set `self.InventoryWindow` _returnvalue)
      (bind _asmy_player_controller (cast `/Game/Blueprints/Char_Blueprints/MyPlayerController` (`GameplayStatics.GetPlayerController` 0)))
      (bind _returnvalue_2 (`CanvasPanel.AddChildToCanvas` (`/Game/Blueprints/InventorySystem/InventoryUI/HUD.HUDCanvas` (`/Game/Blueprints/Char_Blueprints/MyPlayerController.HUDWidget` _asmy_player_controller)) (`self.InventoryWindow`)))
      (`CanvasPanelSlot.SetAutoSize` _returnvalue_2 true)
      (`CanvasPanelSlot.SetAlignment` _returnvalue_2 (0.0 1.0))
      (`CanvasPanelSlot.SetAnchors` _returnvalue_2 (make `Anchors` (0.0 1.0) (0.0 1.0))))))