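; Base pawn that moves and turns in response to the MoveForward and MoveRight input values.
; Each Tick it clamps the input vector to unit length and offsets the capsule in world space by speed and delta time, with sweep for collision.
; Above a small input threshold, it lerps the actor rotation toward the movement direction along the shortest path; otherwise it prints a debug message.
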(event `self.ReceiveTick`
  (params (DeltaSeconds :type "Float (single-precision)"))
  (bind _returnvalue (`KismetMathLibrary.ClampVectorSize` (`KismetMathLibrary.MakeVector` (`self.GetInputAxisValue`) (`self.GetInputAxisValue`)) 0.0 1.0))
  ;[1 1 1] Handle Movement
  (`SceneComponent.K2_AddWorldOffset` (`self.Capsule`) (* (* _returnvalue DeltaSeconds) (`self.MoveSpeed`)) true false)
  (if (> (`KismetMathLibrary.VSize` _returnvalue) 0.1)
    (bind _returnvalue_2 (`self.K2_SetActorRotation` (`KismetMathLibrary.RLerp` (`self.K2_GetActorRotation`) (`KismetMathLibrary.Conv_VectorToRotator` _returnvalue) (* (`self.RotationSpeed`) DeltaSeconds) true)))
    (if _returnvalue_2
      _)
    (else
      (`KismetSystemLibrary.PrintString` "VECTOR==0" true true (struct :`G` 0.66 :`B` 1.0 :`A` 1.0) 0.1))))

(fn `UserConstructionScript`)