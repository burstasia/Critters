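; Base character Blueprint that handles player movement along fixed world axes, independent of camera or actor facing.
; MoveForward and MoveRight axis events feed Add Movement Input on world X and Y respectively.
; An alternative NormalMovement function, never called, sweeps the capsule by clamped input scaled by MoveSpeed and delta time, lerping rotation toward the input direction at RotationSpeed.
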(event `self.ReceiveTick`
  (params (DeltaSeconds :type "Float (single-precision)")))

(event `InputAxis|MoveForward`
  (params (AxisValue :type "Float (single-precision)"))
  (`self.AddMovementInput` (`KismetMathLibrary.MakeVector` 1.0) AxisValue))

(event `InputAxis|MoveRight`
  (params (AxisValue :type "Float (single-precision)"))
  (`self.AddMovementInput` (`KismetMathLibrary.MakeVector` 0.0 1.0) AxisValue))

(fn `NormalMovement`
  (params (DeltaSeconds :type "Float (double-precision)"))
  (bind _returnvalue (`KismetMathLibrary.ClampVectorSize` (`KismetMathLibrary.MakeVector` (`self.GetInputAxisValue`) (`self.GetInputAxisValue`)) 0.0 1.0))
  (`SceneComponent.K2_AddWorldOffset` (`self.CapsuleComponent`) (* (* _returnvalue DeltaSeconds) (`self.moveSpeed`)) true false)
  (if (> (`KismetMathLibrary.VSize` _returnvalue) 0.0)
    (`self.K2_SetActorRotation` (`KismetMathLibrary.RLerp` (`self.K2_GetActorRotation`) (`KismetMathLibrary.Conv_VectorToRotator` _returnvalue) (* (`self.rotationSpeed`) DeltaSeconds) true))))

(fn `UserConstructionScript`)