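; Camera actor that follows the first Base_Char_BP_01 in the level from a raised position.
; A looping near-zero timer, started on BeginPlay, drives UpdateCamera instead of Tick.
; Each update re-finds player controllers and the character, retargets the view to itself and resets spring arm length.
; Position passes through VInterpTo from the stored previous position, with no interp speed set, plus a height offset.
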(event `self.ReceiveBeginPlay`
  (`KismetSystemLibrary.K2_SetTimer` null "UpdateCamera" 0.0001 true))

(event `UpdateCamera`
  (bind _returnvalue (`KismetMathLibrary.MakeVector` (.x (`KismetMathLibrary.VInterpTo` (`self.prevPos`) (`self.newPos`) (`GameplayStatics.GetWorldDeltaSeconds`))) (.y (`KismetMathLibrary.VInterpTo` (`self.prevPos`) (`self.newPos`) (`GameplayStatics.GetWorldDeltaSeconds`))) (+ (.z (`KismetMathLibrary.VInterpTo` (`self.prevPos`) (`self.newPos`) (`GameplayStatics.GetWorldDeltaSeconds`))) 200.0)))
  (bind _outactors (`GameplayStatics.GetAllActorsOfClass` "/Script/Engine.PlayerController"))
  (`PlayerController.SetViewTargetWithBlend` _outactors self 0.0 "VTBlend_Linear" 0.0 false)
  (set `SpringArmComponent.TargetArmLength` 500.0 (`self.SpringArm`))
  (bind _outactors_2 (`GameplayStatics.GetAllActorsOfClass` "/Game/Blueprints/Char_Blueprints/Base_Char_BP_01.Base_Char_BP_01_C"))
  (set `self.newPos` (`self.K2_GetActorLocation` (`|GetArrayItem` _outactors_2)))
  (`self.K2_SetActorLocation` _returnvalue)
  (set `self.prevPos` _returnvalue))

(fn `UserConstructionScript`)